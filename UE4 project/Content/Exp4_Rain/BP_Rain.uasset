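; BP_Rain controls a rain effect that pairs a particle system with either OSC-driven sound or a sampled audio track.
; Start and Reset switch the particles and send toggle messages over OSC, with Reset also zeroing intensity.
; PlaySampled instead toggles the Pioggia audio together with the particles.
; ObtainSliderValue maps one slider value to scaled OSC intensity and interpolated particle fall velocity and spawn count.
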(event `/Game/StartInterface.Start`
  (`ActorComponent.Activate` (`self.ParticleSystemComponent`) false)
  (`OscFunctionLibrary.SendOsc` "/toggle" (`OscFunctionLibrary.PushInt` :`Value` 1) 4))

(event `/Game/StartInterface.Reset`
  (`ActorComponent.Deactivate` (`self.ParticleSystemComponent`))
  (`OscFunctionLibrary.SendOsc` "/toggle" (`OscFunctionLibrary.PushInt` _) 4)
  (`OscFunctionLibrary.SendOsc` "/intensity" (`OscFunctionLibrary.PushFloat` _) 4))

(event `/Game/StartInterface.PlaySampled`
  (bind _particlesystemcomponent (`self.ParticleSystemComponent`))
  (bind _pioggia (`self.Pioggia`))
  (if (`AudioComponent.IsPlaying` (`self.Pioggia`))
    (`AudioComponent.Stop` _pioggia)
    (`ActorComponent.Deactivate` _particlesystemcomponent)
    (else
      (`AudioComponent.Play` _pioggia 0.0)
      (`ActorComponent.Activate` _particlesystemcomponent false))))

(fn `ObtainSliderValue`
  (params (Value :type "Float (double-precision)"))
  (bind _particlesystemcomponent (`self.ParticleSystemComponent`))
  (`OscFunctionLibrary.SendOsc` "/intensity" (`OscFunctionLibrary.PushFloat` :`Value` (* Value 0.7)) 4)
  (`ParticleSystemComponent.SetVectorParameter` _particlesystemcomponent "RainVelocity" (`KismetMathLibrary.MakeVector` 0.0 0.0 (`KismetMathLibrary.Lerp` -600.0 -1300.0 Value)))
  (`ParticleSystemComponent.SetVectorParameter` _particlesystemcomponent "SpawnNumber" (`KismetMathLibrary.MakeVector` 0.0 0.0 (`KismetMathLibrary.Lerp` 400.0 800.0 Value))))

(fn `UserConstructionScript`)