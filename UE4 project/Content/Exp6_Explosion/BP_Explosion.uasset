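; BP_Explosion is an explosion effect that pairs a particle burst with either sampled audio or an OSC trigger.
; PlaySampled plays the Audio component, while Start sends /explTrigger over OSC instead, and both then activate the particle system.
; The construction script sends a default /blastTime over OSC, and ObtainSliderValue rescales a slider value to update it on the same target.
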(event `/Game/StartInterface.PlaySampled`
  (`AudioComponent.Play` (`self.Audio`) 0.0)
  (`ActorComponent.Activate` (`self.Particle_Explosion`) true :!label _label))

(event `/Game/StartInterface.Start`
  (`OscFunctionLibrary.SendOsc` "/explTrigger" (`OscFunctionLibrary.PushInt` :`Value` 1) 6)
  (goto _label))

(fn `Obtain Slider Value`
  (params (Value :type "Float (double-precision)"))
  (`OscFunctionLibrary.SendOsc` "/blastTime" (`OscFunctionLibrary.PushFloat` :`Value` (+ (* Value 0.15) 0.05)) 6))

(fn `UserConstructionScript`
  (`OscFunctionLibrary.SendOsc` "/blastTime" (`OscFunctionLibrary.PushFloat` :`Value` 0.05) 6))