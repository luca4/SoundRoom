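; BP_Handgun is a handgun that fires a small physics projectile with an explosion effect at its muzzle.
; Two events share the firing logic: Start first sends an OSC "/shoot" message, while PlaySampled plays the local Sparo component instead.
; Both spawn BP_Projectile at BulletShooter and push it with a fixed force along world X, regardless of the gun's rotation.
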(event `/Game/StartInterface.Start`
  (`OscFunctionLibrary.SendOsc` "/shoot" (`OscFunctionLibrary.PushInt` :`Value` 1) 1)
  (bind _returnvalue (`|SpawnActorFromClass` "/Game/Exp2_Handgun/BP_Projectile.BP_Projectile_C" (`KismetMathLibrary.MakeTransform` (`SceneComponent.K2_GetComponentLocation` (`self.bullet shooter`)) (struct) (0.04 0.04 0.04)) "AdjustIfPossibleButAlwaysSpawn" "OverrideRootScale" self null :!label _label))
  (`PrimitiveComponent.AddForce` (`/Game/Exp2_Handgun/BP_Projectile.Projectile` _returnvalue) (300000.0 0.0 0.0) "None" true)
  (`GameplayStatics.SpawnEmitterAtLocation` "/Game/StarterContent/Particles/P_Explosion.P_Explosion" (`SceneComponent.K2_GetComponentLocation` (`self.bullet shooter`)) (struct) (0.2 0.2 0.2)))

(event `/Game/StartInterface.PlaySampled`
  (`AudioComponent.Play` (`self.Sparo`) 0.0)
  (goto _label))

(fn `UserConstructionScript`)