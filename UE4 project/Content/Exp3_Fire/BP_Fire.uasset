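; BP_Fire is a fire effect that pairs a particle system with either OSC-driven sound or sampled audio.
; Start and Reset toggle the particles and send OSC on/off messages for flame and crackles to an external target.
; PlaySampled instead toggles the Fuoco audio together with the particles.
; The construction script sends a base crackle frequency, which ObtainSliderValue raises linearly with the slider value.
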(event `/Game/StartInterface.Start`
  (bind _output (`OscFunctionLibrary.PushInt` :`Value` 1))
  (`ActorComponent.Activate` (`self.ParticleSystemComponent`) false)
  (`OscFunctionLibrary.SendOsc` "/flameOnOff" _output 2)
  (`OscFunctionLibrary.SendOsc` "/crackles/OnOff" _output 2))

(event `/Game/StartInterface.Reset`
  (bind _output (`OscFunctionLibrary.PushInt` _))
  (`ActorComponent.Deactivate` (`self.ParticleSystemComponent`))
  (`OscFunctionLibrary.SendOsc` "/flameOnOff" _output 2)
  (`OscFunctionLibrary.SendOsc` "/crackles/OnOff" _output 2))

(event `/Game/StartInterface.PlaySampled`
  (bind _particlesystemcomponent (`self.ParticleSystemComponent`))
  (bind _fuoco (`self.Fuoco`))
  (if (`AudioComponent.IsPlaying` (`self.Fuoco`))
    (`AudioComponent.Stop` _fuoco)
    (`ActorComponent.Deactivate` _particlesystemcomponent)
    (else
      (`AudioComponent.Play` _fuoco 0.0)
      (`ActorComponent.Activate` _particlesystemcomponent false))))

(fn `ObtainSliderValue`
  (params (Value :type "Float (double-precision)"))
  (`OscFunctionLibrary.SendOsc` "/crackles/freq" (`OscFunctionLibrary.PushFloat` :`Value` (+ (* Value 80.0) 120.0)) 2))

(fn `UserConstructionScript`
  (`OscFunctionLibrary.SendOsc` "/crackles/freq" (`OscFunctionLibrary.PushFloat` :`Value` 120.0) 2))